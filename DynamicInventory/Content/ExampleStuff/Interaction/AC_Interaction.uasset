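; Character component that finds the interactible actor in the player's view and triggers interaction with it.
; On the locally controlled character, a looping timer is set up, presumably driving FindTarget's sphere trace from the eyes along the third-person camera's forward vector.
; SetNewTarget sends targeted on/off interface messages and binds to target destruction.
; Interact messages the target locally for potential prediction, then relays through a server event.
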(event Custom|Server_Interact
  (params (Actor :type Actor%20Object%20Reference))
  (Class|INInteractible|ServerInteraction(Message) Actor (Variables|ACInteraction|GetOwningCharacter)))

(event EventBeginPlay
  (|CallParentFunction)
  (bind _ascharacter (Utilities|Casting|CastToCharacter (Components|GetOwner)))
  (bind _output_get (Variables|ACInteraction|SetOwningCharacter _ascharacter))
  (if (Pawn|IsLocallyControlled _output_get)
    (Utilities|Time|SetTimerbyEvent (EventDispatchers|CreateEvent :!event FindTarget) 0.2 true)))

(fn FindTarget
  (bind _owningcharacter (Variables|ACInteraction|GetOwningCharacter))
  (bind _outlocation (Actor|GetActorEyesViewPoint _owningcharacter))
  (bind _asbp_third_person_character (Utilities|Casting|CastToBP_ThirdPersonCharacter (Variables|ACInteraction|GetOwningCharacter)))
  (bind (_outhit _returnvalue) (Collision|SphereTraceByChannel _outlocation (+ _outlocation (* (Math|Vector|GetForwardVector (Variables|/DynamicInventory/ExampleStuff/BP_ThirdPersonCharacter.BP_ThirdPersonCharacter_C|GetFollowCamera _asbp_third_person_character)) (Variables|Settings|GetInteractionDistance))) (Variables|Settings|GetInteractionRadius) "TraceTypeQuery1" false (Utilities|Array|MakeArray (Variables|ACInteraction|GetOwningCharacter)) (Variables|Settings|GetInteractionDebugTrace)))
  (if _returnvalue
    (bind _isinteractible (Class|INInteractible|IsInteractible(Message) (.HitActor (Collision|BreakHitResult _outhit))))
    (if _isinteractible
      (if (!= (Variables|ACInteraction|GetCurrentTarget) (.HitActor (Collision|BreakHitResult _outhit)))
        (ACInteraction|SetNewTarget (.HitActor (Collision|BreakHitResult _outhit))))
      (else
        (Utilities|IsValid (Variables|ACInteraction|GetCurrentTarget) :!label _label
          (:Is%20Valid
            (ACInteraction|SetNewTarget)))))
    (else
      (goto _label))))

(fn SetNewTarget
  (params (NewTarget :type Actor%20Object%20Reference))
  (Utilities|IsValid (Variables|ACInteraction|GetCurrentTarget)
    (:Is%20Valid
      (Class|INInteractible|SetTargeted(Message) (Variables|ACInteraction|GetCurrentTarget) false))
    (:Is%20Not%20Valid
      _))
  (bind _output_get (Variables|ACInteraction|SetCurrentTarget NewTarget))
  (Utilities|IsValid _output_get
    (:Is%20Valid
      (Class|INInteractible|SetTargeted(Message) _output_get true)
      (Game|BindEventtoOnDestroyed _output_get (EventDispatchers|CreateEvent :!event OnCurrentTargetDestroyed)))))

(fn Interact
  (bind _currenttarget (Variables|ACInteraction|GetCurrentTarget))
  ;[1 0 1 0.5072] Doing client interaction for potential prediction shit
  (Class|INInteractible|ClientInteraction(Message) _currenttarget (Variables|ACInteraction|GetOwningCharacter))
  (CallFunction|ServerInteract _currenttarget))

(fn OnCurrentTargetDestroyed
  (params (DestroyedActor :type Actor%20Object%20Reference))
  (ACInteraction|SetNewTarget))