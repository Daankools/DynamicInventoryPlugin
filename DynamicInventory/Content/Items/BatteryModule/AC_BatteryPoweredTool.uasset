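; Item module component that gives a tool a battery, tracking charge and active state and saving both into the item's instanced struct.
; While the tool is active, a looping timer drains charge; an empty battery switches it off and blocks reactivation.
; The replicated level updates a battery HUD widget through OnRep, created only for the locally controlled owner while equipped.
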(event EventBeginPlay
  ;[1 0 1 0.5072] Hud widgets for battery
  (if (and (Pawn|IsLocallyControlled (Variables|/Script/Engine.Actor|GetInstigator (Components|GetOwner))) (Variables|Settings|GetIsEquipped))
    (bind _returnvalue (UserInterface|CreateWidget "/DynamicInventory/Items/BatteryModule/WBP_ItemModule_BatteryState.WBP_ItemModule_BatteryState_C"))
    (bind _output_get (Variables|ACBatteryPoweredTool|SetBatteryWidget _returnvalue))
    (UserInterface|Viewport|AddtoViewport _output_get 0)
    (Utilities|IsValid (Variables|ACBatteryPoweredTool|GetBatteryWidget)
      (:Is%20Valid
        (Default|UpdateBatteryValue (Variables|ACBatteryPoweredTool|GetBatteryWidget) (Variables|ACBatteryPoweredTool|GetCurrentBatteryLevel))
        (|CallParentFunction))
      (:Is%20Not%20Valid
        (|CallParentFunction)))
    (else
      (|CallParentFunction))))

(event EventEndPlay
  (params (EndPlayReason :type EEndPlayReason%20Enum :default "Destroyed"))
  ;[1 0 1 0.5072] Hud widgets for battery
  (|CallParentFunction EndPlayReason)
  (if (and (Pawn|IsLocallyControlled (Variables|/Script/Engine.Actor|GetInstigator (Components|GetOwner))) (Variables|Settings|GetIsEquipped))
    (Widget|RemovefromParent (Variables|ACBatteryPoweredTool|GetBatteryWidget))))

(fn SetCurrentBatteryLevel
  (params (CurrentBatteryLevel :type Float%20%28double-precision%29))
  ;[1 1 0 0.5] Server: set the battery level. Repnotify it for visual updates.
  (bind _output_get (Variables|ACBatteryPoweredTool|SetCurrentBatteryLevel CurrentBatteryLevel))
  (if (and (<= _output_get 0.0) (Utilities|Enum|Equal(Enum) (Variables|ACBatteryPoweredTool|GetToolActive) "NewEnumerator2"))
    (ACBatteryPoweredTool|SetToolActive "NewEnumerator1")))

(fn InitializeModule
  (params (ItemModule :type Array%20of%20Instanced%20Struct%20Structures))
  (|CallParentFunction ItemModule)
  (for (_array_element _array_index) ItemModule
    (bind _value (Utilities|InstancedStruct|GetInstancedStructValue _array_element)
      (:Valid
        (Variables|Default|SetStructIndex _array_index)
        (ACBatteryPoweredTool|SetCurrentBatteryLevel (.CurrentBattery (Utilities|Struct|BreakSTR_ItemState_Battery _value)))
        (ACBatteryPoweredTool|SetToolActive (.ToolActivateState (Utilities|Struct|BreakSTR_ItemState_Battery _value)))
        (return))
      (:NotValid
        (return)))))

(fn DepleteBattery
  (params (DepleteBattery :type Float%20%28double-precision%29))
  (ACBatteryPoweredTool|SetCurrentBatteryLevel (- (Variables|ACBatteryPoweredTool|GetCurrentBatteryLevel) DepleteBattery)))

(fn ModifyStruct
  (bind _returnvalue (Utilities|InstancedStruct|MakeInstancedStruct (Utilities|Struct|MakeSTR_ItemState_Battery (Variables|ACBatteryPoweredTool|GetCurrentBatteryLevel) (Variables|ACBatteryPoweredTool|GetToolActive))))
  (return _returnvalue))

(fn OnRepCurrentBatteryLevel
  (bind _batterywidget (Variables|ACBatteryPoweredTool|GetBatteryWidget))
  (if (Pawn|IsLocallyControlled (Variables|/Script/Engine.Actor|GetInstigator (Components|GetOwner)))
    (Utilities|IsValid _batterywidget
      (:Is%20Valid
        (Default|UpdateBatteryValue _batterywidget (Variables|ACBatteryPoweredTool|GetCurrentBatteryLevel))))))

(fn SetToolActive
  (params (FlashlightActive :type EN_ToolActiveState%20Enum :default "NewEnumerator0"))
  (if (not (and (<= (Variables|ACBatteryPoweredTool|GetCurrentBatteryLevel) 0.0) (Utilities|Enum|Equal(Enum) FlashlightActive "NewEnumerator2")))
    (Variables|ACBatteryPoweredTool|SetToolActive FlashlightActive)
    (Default|CallOnToolActivated FlashlightActive)
    (if (Utilities|Enum|Equal(Enum) FlashlightActive "NewEnumerator2")
      (bind _returnvalue (Utilities|Time|SetTimerbyEvent (EventDispatchers|CreateEvent :!event DrainBattery) (Variables|Settings|GetBatteryDrainInterval) true))
      (Variables|ACBatteryPoweredTool|SetBatteryDrainTimer _returnvalue)
      (else
        (Utilities|Time|ClearandInvalidateTimerbyHandle (Variables|ACBatteryPoweredTool|GetBatteryDrainTimer))))))

(fn DrainBattery
  (ACBatteryPoweredTool|DepleteBattery (Variables|Settings|GetBatteryDrainAmount)))

(fn EndModule
  ;[1 1 0 0.5] Server: Cleanup
  (Utilities|Time|ClearandInvalidateTimerbyHandle (Variables|ACBatteryPoweredTool|GetBatteryDrainTimer))
  (|CallParentFunction))