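; Base actor component for item modules that load and persist their slice of an item's state.
; On BeginPlay it caches the owning ItemBase's GUID, and on authority passes that item's ItemStates from ItemRegistrySubsystem to InitializeModule.
; On EndPlay, except when ending play in editor, it writes ModifyStruct's result back to the registry at StructIndex.
; Child modules override InitializeModule and ModifyStruct to read and supply their own struct data.
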(event EventBeginPlay
  (|CallParentFunction)
  (ACItemModuleBase|SetGUIDReference)
  (Networking|SwitchHasAuthority
    (:Authority
      (ACItemModuleBase|InitializeModule (Utilities|Struct|BreakItemInstance (Class|ItemRegistrySubsystem|GetItem (Subsystems|GetItemRegistrySubsystem) (Variables|ACItemModuleBase|GetOwningItemRef)))))))

(event EventEndPlay
  (params (EndPlayReason :type EEndPlayReason%20Enum :default "Destroyed"))
  (|CallParentFunction EndPlayReason)
  (if (Utilities|Enum|NotEqual(Enum) EndPlayReason "EndPlayInEditor")
    (ACItemModuleBase|EndModule)))

(fn InitializeModule
  (params (ItemModule :type Array%20of%20Instanced%20Struct%20Structures))
  ;[1 1 0 0.5] Server: OVERRIDE this function. Grab the structs you need for the module and output the data into variables/functions. See the battery module example.
)

(fn EndModule
  (bind _outputstruct (ACItemModuleBase|ModifyStruct))
  (Class|ItemRegistrySubsystem|SetItemState (Subsystems|GetItemRegistrySubsystem) (Variables|ACItemModuleBase|GetOwningItemRef) (Variables|ACItemModuleBase|GetStructIndex) _outputstruct)
  (return))

(fn ModifyStruct
  ;[1 1 0 0.5] Server: Override and provide the struct data you need.
  (return ""))

(fn SetGUIDReference
  (bind _asitem_base (Utilities|Casting|CastToItemBase (Components|GetOwner)))
  (Variables|ACItemModuleBase|SetOwningItemRef (Variables|/Script/DynamicInventory.ItemBase|GetItemGuid _asitem_base)))