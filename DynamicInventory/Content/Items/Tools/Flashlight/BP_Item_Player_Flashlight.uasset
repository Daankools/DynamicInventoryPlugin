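; Player flashlight tool item that is held in the left hand and casts a spotlight while active.
; It extends a parent item class, with both owner and remote attach hooks snapping it to the instigator character's mesh at the HandGrip_L socket.
; The replicated tool active state handler toggles SpotLight visibility on all clients, showing it only in the On state.
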(fn ConstructionScript
  (|CallParentFunction))

(fn AttachItemOwner
  (|CallParentFunction)
  (bind _ascharacter (Utilities|Casting|CastToCharacter (Game|GetInstigator)))
  (Transformation|AttachComponentToComponent (Variables|/Script/Engine.Character|GetMesh _ascharacter) "HandGrip_L" "SnapToTarget" "SnapToTarget" "KeepWorld" false))

(fn ActualonRepToolActiveState
  (params (ToolActiveState :type EN_ToolActiveState%20Enum :default "NewEnumerator0"))
  ;[0 0 0 0.5] ON ALL CLIENTS: If activation changes, change the light visibility
  (|CallParentFunction ToolActiveState)
  (Rendering|SetVisibility (Variables|Default|GetSpotLight) (Utilities|Select :Index (Variables|Default|GetToolActiveState) :NewEnumerator0 false :NewEnumerator1 false :NewEnumerator2 true) false))

(fn AttachItemRemote
  (|CallParentFunction)
  (bind _ascharacter (Utilities|Casting|CastToCharacter (Game|GetInstigator)))
  (Transformation|AttachComponentToComponent (Variables|/Script/Engine.Character|GetMesh _ascharacter) "HandGrip_L" "SnapToTarget" "SnapToTarget" "KeepWorld" false))