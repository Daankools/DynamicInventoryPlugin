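; World version of the flashlight tool item, a pickup that players can collect into their inventory.
; Server interaction adds its item GUID to the AC_Inventory on the character's PlayerState and destroys the actor; client interaction does nothing.
; The replicated tool active state drives SpotLight visibility on all clients, lit only when On.
; It is always interactible and swaps the mesh material as a highlight while targeted.
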(fn ConstructionScript
  (|CallParentFunction))

(fn ActualonRepToolActiveState
  (params (ToolActiveState :type EN_ToolActiveState%20Enum :default "NewEnumerator0"))
  ;[0 0 0 0.5] ON ALL CLIENTS: If activation changes, change the light visibility
  (|CallParentFunction ToolActiveState)
  (Rendering|SetVisibility (Variables|Default|GetSpotLight) (Utilities|Select :Index (Variables|Default|GetToolActiveState) :NewEnumerator0 false :NewEnumerator1 false :NewEnumerator2 true) false))

(fn ClientInteraction
  (params (Character :type Character%20Object%20Reference))
  (return false))

(fn IsInteractible
  (return true true))

(fn ServerInteraction
  (params (Character :type Character%20Object%20Reference))
  (Default|AddItemtoInventory (Actor|GetComponentbyClass (Variables|/Script/Engine.Pawn|GetPlayerState Character) "/DynamicInventory/Inventory/AC_Inventory.AC_Inventory_C") (Variables|Default|GetItemGuid))
  (Actor|DestroyActor)
  (return true))

(fn SetTargeted
  (params (Targeted :type Boolean))
  (Rendering|Material|SetMaterial (Variables|Default|GetStaticMesh) 0 (select Targeted "/Engine/MapTemplates/Materials/BasicAsset01.BasicAsset01" "/Engine/BasicShapes/BasicShapeMaterial.BasicShapeMaterial"))
  (return true))