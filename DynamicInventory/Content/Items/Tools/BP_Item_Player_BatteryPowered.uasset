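; Base battery-powered player tool item whose primary interaction toggles its AC_BatteryPoweredTool component between on and off on the server.
; The component's activation event sets a replicated ToolActiveState, whose OnRep calls an empty overridable function on all clients, since a normal OnRep can't be overridden.
; Children put their on/off logic in that override.
; Unequipping ends the component's module on the server so its data gets saved.
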(event OnToolActivated(AC_BatteryPoweredTool)
  (params (State :type EN_ToolActiveState%20Enum :default "NewEnumerator0"))
  ;[1 1 0 0.5] SERVER: When the item is toggled on or off. (Expand the ENUM if you want more states).
  (Variables|BPItemPlayerBatteryPowered|SetToolActiveState State))

(event EventStartPrimaryInteraction
  (bind _ac_batterypoweredtool (Variables|Default|GetAC_BatteryPoweredTool))
  ;[1 1 0 0.5] Server: Interaction
  (switch Utilities|FlowControl|Switch|SwitchonEN_ToolActiveState (Variables|/DynamicInventory/Items/BatteryModule/AC_BatteryPoweredTool.AC_BatteryPoweredTool_C|GetToolActive _ac_batterypoweredtool)
    (:NewEnumerator0
      (Default|SetToolActive _ac_batterypoweredtool "NewEnumerator2" :!label _label))
    (:NewEnumerator1
      (goto _label))
    (:NewEnumerator2
      (Default|SetToolActive _ac_batterypoweredtool "NewEnumerator1"))))

(event EventSetEquipItem
  (params (Equip :type Boolean))
  ;[1 1 0 0.5] SERVER: End the current module so that data gets saved.
  (|CallParentFunction Equip)
  (if (not Equip)
    (Default|EndModule (Variables|Default|GetAC_BatteryPoweredTool))))

(fn ConstructionScript
  (|CallParentFunction))

(fn ActualonRepToolActiveState
  (params (ToolActiveState :type EN_ToolActiveState%20Enum :default "NewEnumerator0"))
  ;[0 0 0 0.5] OVERRIDE: this event is fired whenever the active state of the tool changes. So use this to trigger whatever logic should happen. Keep in mind; this is running on all clients.
)

(fn OnRepToolActiveState
  ;[0 0 0 0.5] RUNNING ON ALL: The "Actual on rep" is called because a normal OnRep can't be overridden.
  (BPItemPlayerBatteryPowered|ActualonRepToolActiveState (Variables|BPItemPlayerBatteryPowered|GetToolActiveState)))