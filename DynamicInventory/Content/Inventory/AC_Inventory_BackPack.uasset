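; Backpack inventory component on the PlayerState that shows and hides the player's backpack screen and handles dropping items.
; Opening resolves each inventory entry through the item cache and item-definition lookup, appends it to a backpack array, and feeds that to a new backpack widget.
; Mouse cursor and input mode switch between game-and-UI and game-only as it opens and closes.
; A server event drops the selected item by GUID.
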(event Custom|Server_DropButtonSelected
  (params (GUID :type Guid%20Structure))
  (CallFunction|DropItem GUID))

(fn SetInventoryOpen
  (params (Open :type Boolean))
  ;[1 0 1 0.5] Open my backpack
  (|CallParentFunction Open)
  (if Open
    ;;[0.15 0.15 0.15 0.5] Create the backpack array and intiliaze the widget
    (for _array_element (Variables|Default|GetInventory)
      (bind _foundinstance (CallFunction|FindIteminCache _array_element))
      (bind _itemdefinition (CallFunction|GetItembyID (Utilities|Struct|BreakItemInstance _foundinstance)))
      (Utilities|Array|Add (LocalVariables|GetBackpack) (Utilities|Struct|MakeSTR_BackPackEntry _array_element _itemdefinition)))
    (bind _returnvalue (UserInterface|CreateWidget "/DynamicInventory/Inventory/WBP_Inventory_Backpack.WBP_Inventory_Backpack_C" 0 (LocalVariables|GetBackpack)))
    (bind _output_get (Variables|ACInventoryBackpack|SetInventoryWidget _returnvalue))
    (UserInterface|Viewport|AddtoViewport _output_get 0)
    (bind _asplayer_state (Utilities|Casting|CastToPlayerState (Components|GetOwner)))
    (Variables|/Script/Engine.PlayerController|SetbShowMouseCursor (Game|GetPlayerController _asplayer_state) true)
    (Input|SetInputModeGameandUI (Game|GetPlayerController _asplayer_state) 0 "DoNotLock" true true)
    (else
      ;;[0.15 0.15 0.15 0.5] Remove widget
      (Widget|RemovefromParent (Variables|ACInventoryBackpack|GetInventoryWidget))
      (Variables|ACInventoryBackpack|SetInventoryWidget 0)
      (bind _asplayer_state_2 (Utilities|Casting|CastToPlayerState (Components|GetOwner)))
      (Variables|/Script/Engine.PlayerController|SetbShowMouseCursor (Game|GetPlayerController _asplayer_state_2) false)
      (Input|SetInputModeGameOnly (Game|GetPlayerController _asplayer_state_2) true))))